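; Game mode that handles linear level progression and game completion.
; On BeginPlay it sets game-only input and looks up the current level in the Levels array to cache the following one, or "End" when none follows.
; LevelComplete shows a completion widget, then a short timer calls LoadNextLevel, which opens that level or shows the game-complete screen with UI-only input.
; EndGame opens the Main1 level.
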(event `self.ReceiveBeginPlay`
  (bind _returnvalue (`GameplayStatics.GetPlayerController` 0))
  (bind _levels (`self.Levels`))
  (bind _returnvalue_2 (- (`KismetArrayLibrary.Array_Length` _levels) 1))
  (set `PlayerController.bShowMouseCursor` false _returnvalue)
  (`WidgetBlueprintLibrary.SetInputMode_GameOnly` _returnvalue)
  (bind _returnvalue_3 (`GameplayStatics.GetCurrentLevelName` true))
  (for (_array_element _array_index) _levels :!label _label
    (set `self.currentIndex` _array_index)
    (if (and (`KismetStringLibrary.EqualEqual_StrStr` _array_element _returnvalue_3) (< (`self.currentIndex`) _returnvalue_2))
      (set `self.nextLevel` (`|GetArrayItem` (`self.Levels`) (+ (`self.currentIndex`) 1)))
      (`self.break loop`)
      (elif (== (`self.currentIndex`) _returnvalue_2)
        (set `self.nextLevel` "End")
        (`self.break loop`)))))

(event `break loop`
  (goto _label :!via `Break`))

(fn `EndGame`
  (`GameplayStatics.OpenLevel` "Main1"))

(fn `LevelComplete`
  (bind _returnvalue (`|CreateWidget` "/Game/Blueprints/WBP_LevelComplete.WBP_LevelComplete_C"))
  (`UserWidget.AddToViewport` _returnvalue 0)
  (`KismetSystemLibrary.K2_SetTimer` null "LoadNextLevel" 2.0))

(fn `LoadNextLevel`
  (bind _returnvalue (`GameplayStatics.GetPlayerController` 0))
  (if (`KismetStringLibrary.EqualEqual_StrStr` (`self.nextLevel`) "End")
    (bind _returnvalue_2 (`|CreateWidget` "/Game/Blueprints/WBP_GameComplete.WBP_GameComplete_C"))
    (`UserWidget.AddToViewport` _returnvalue_2 0)
    (set `PlayerController.bShowMouseCursor` true _returnvalue)
    (`WidgetBlueprintLibrary.SetInputMode_UIOnlyEx` _returnvalue _returnvalue_2)
    (else
      (`GameplayStatics.OpenLevel` (`KismetStringLibrary.Conv_StringToName` (`self.nextLevel`))))))

(fn `UserConstructionScript`)